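; AI character that uses AI Perception to track actors tagged EvilPlayer and store them as a Blackboard follow target.
; A stimulus-filtering macro sorts perception updates into sensed, lost or ignored.
; A sensed target is written to the Blackboard and cancels the memory timer.
; A lost target starts that timer, which clears the Blackboard key after the memory duration, giving short-term memory before forgetting.
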(event `self.AIPerception.OnTargetPerceptionUpdated`
  (params (Actor :type "Actor Object Reference") (Stimulus :type "AIStimulus Structure"))
  (`self.ProcessStimuli` Actor Stimulus
    (:`FollowNewActor`
      (`self.FollowNewActorTarget` Actor)
      (`KismetSystemLibrary.PrintString` "Follow New Actor"))
    (:`LostTrackTarget`
      (`self.LostTrackTarget`))))

(fn `FollowNewActorTarget`
  (params (TargetToFollow :type "Object Object Reference"))
  (`KismetSystemLibrary.K2_ClearAndInvalidateTimerHandle` (`self.MemoryDurationTImer`))
  (`BlackboardComponent.SetValueAsObject` (`AIBlueprintHelperLibrary.GetBlackboard` null) (`self.FollowTargetKey`) TargetToFollow)
  (return))

(fn `ForgetAboutTarget`
  (`BlackboardComponent.SetValueAsObject` (`AIBlueprintHelperLibrary.GetBlackboard` null) (`self.FollowTargetKey`) null)
  (return))

(fn `LostTrackTarget`
  (locals (`Memory Duration` :type "Float (single-precision)" :default 1.0))
  (bind _returnvalue (`KismetSystemLibrary.K2_SetTimer` null "ForgetAboutTarget" (`local.Memory Duration`)))
  (set `self.MemoryDurationTImer` _returnvalue)
  (return))

(fn `UserConstructionScript`)